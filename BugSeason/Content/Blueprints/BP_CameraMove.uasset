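; BP_CameraMove is a trigger volume that switches the bug player's camera while the character is inside its box.
; On overlap begin, it blends the BP_BugController's view target to the level's BpC_BugCameraStationary, and on overlap end, back to BpC_BugCamera.
; Both cameras are looked up by class with GetActorOfClass, so each blend uses the first instance found, over CameraBlendTime.
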(event `self.Box.OnComponentBeginOverlap`
  (params (OverlappedComponent :type "PrimitiveComponent Object Reference") (OtherActor :type "Actor Object Reference") (OtherComp :type "PrimitiveComponent Object Reference") (OtherBodyIndex :type Integer) (bFromSweep :type Boolean) (SweepResult :type "HitResult Structure (by ref)"))
  (bind _asbp_bug_character (cast `/Game/Blueprints/Player/BP_BugCharacter` OtherActor))
  (if (`KismetSystemLibrary.IsValid` _asbp_bug_character)
    (bind _asbp_bug_controller (cast `/Game/Blueprints/Player/BP_BugController` (`Pawn.GetController` _asbp_bug_character)))
    (if (`KismetSystemLibrary.IsValid` _asbp_bug_controller)
      (bind _returnvalue (`GameplayStatics.GetActorOfClass` "/Game/Blueprints/Player/BpC_BugCameraStationary.BpC_BugCameraStationary_C"))
      (`PlayerController.SetViewTargetWithBlend` _asbp_bug_controller _returnvalue (`self.CameraBlendTime`) "VTBlend_Linear" 0.0 false))))

(event `self.Box.OnComponentEndOverlap`
  (params (OverlappedComponent :type "PrimitiveComponent Object Reference") (OtherActor :type "Actor Object Reference") (OtherComp :type "PrimitiveComponent Object Reference") (OtherBodyIndex :type Integer))
  (bind _asbp_bug_character (cast `/Game/Blueprints/Player/BP_BugCharacter` OtherActor))
  (if (`KismetSystemLibrary.IsValid` _asbp_bug_character)
    (bind _asbp_bug_controller (cast `/Game/Blueprints/Player/BP_BugController` (`Pawn.GetController` _asbp_bug_character)))
    (if (`KismetSystemLibrary.IsValid` _asbp_bug_controller)
      (bind _returnvalue (`GameplayStatics.GetActorOfClass` "/Game/Blueprints/Player/BpC_BugCamera.BpC_BugCamera_C"))
      (`PlayerController.SetViewTargetWithBlend` _asbp_bug_controller _returnvalue (`self.CameraBlendTime`) "VTBlend_Linear" 0.0 false))))

(fn `UserConstructionScript`)
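; Pushable cube that slides one step along its dominant local X or Y axis, away from a grounded BP_BugCharacter that hits it.
; A distance-scaled timeline drives the slide, with box traces reversing it on obstacles and attaching any BP_MovableLeaf in the path.
; When stopped, it releases the leaf and traces down for water, sinking and disabling further pushes if found.
; Unset move distances default to the box's size.
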(event `self.ReceiveBeginPlay`
  (bind (_move_amount_x _move_amount_y _move_amount_z) (`KismetMathLibrary.BreakVector` (`self.Move Amount`)))
  (bind (_move_amount_x_2 _move_amount_y_2 _move_amount_z_2) (`KismetMathLibrary.BreakVector` (`self.Move Amount`)))
  (bind (_returnvalue_x _returnvalue_y _returnvalue_z) (`KismetMathLibrary.BreakVector` (* (`BoxComponent.GetUnscaledBoxExtent` (`self.Box`)) (2.0 2.0 2.0))))
  ;[1 1 1] Yes, I Know This Is Really Ugly Code
  (`|ExecutionSequence`
    (:`then_0`
      (if (== _move_amount_x 0.0)
        (set `self.Move Amount` (`KismetMathLibrary.MakeVector` _returnvalue_x _move_amount_y_2 _move_amount_z_2))))
    (:`then_1`
      (if (== _move_amount_y 0.0)
        (set `self.Move Amount` (`KismetMathLibrary.MakeVector` _move_amount_x_2 _returnvalue_y _move_amount_z_2))))
    (:`then_2`
      (if (== _move_amount_z 0.0)
        (set `self.Move Amount` (`KismetMathLibrary.MakeVector` _move_amount_x_2 _move_amount_y_2 _returnvalue_z))))))

(event `self.ReceiveHit`
  (params (MyComp :type "PrimitiveComponent Object Reference") (Other :type "Actor Object Reference") (OtherComp :type "PrimitiveComponent Object Reference") (bSelfMoved :type Boolean) (HitLocation :type "Vector Structure") (HitNormal :type "Vector Structure") (NormalImpulse :type "Vector Structure") (Hit :type "HitResult Structure (by ref)"))
  ;[1 1 1] Make Sure We Hit Bug
  (bind _asbp_bug_character (cast `/Game/Blueprints/Player/BP_BugCharacter` Other))
  (if (and (`NavMovementComponent.IsMovingOnGround` (`Character.CharacterMovement` _asbp_bug_character)) (== (`GameplayStatics.GetObjectClass` OtherComp) "/Script/Engine.CapsuleComponent"))
    (`self.Move Cube` (`self.K2_GetActorLocation` Other))))

(event `Move Cube`
  (params (`Away Location` :type "Vector Structure"))
  (bind (_move_amount_x _move_amount_y) (`KismetMathLibrary.BreakVector` (`self.Move Amount`)))
  (bind (_returnvalue_x _returnvalue_y) (`KismetMathLibrary.BreakVector` (`KismetMathLibrary.InverseTransformLocation` (`self.GetTransform`) `Away Location`)))
  (bind _returnvalue (> (`KismetMathLibrary.Abs` _returnvalue_x) (`KismetMathLibrary.Abs` _returnvalue_y)))
  (bind _returnvalue_2 (* (`KismetMathLibrary.FClamp` (* -1.0 (select `bool` _returnvalue :`false` _returnvalue_y :`true` _returnvalue_x)) -1.0) (select `bool` _returnvalue :`false` _move_amount_y :`true` _move_amount_x)))
  ;[1 1 1] Finding Variables Based On Position
  (if (`self.CanMove`)
    (`/Engine/EditorBlueprintResources/StandardMacros.DoOnce` false :!label _label
      (:`Completed`
        ;[1 1 1] Box Tracing and Setting Location
        (`|ExecutionSequence`
          (:`then_0`
            (bind (_return_start _return_end) (`self.Set Playrate And Variables` (`self.MoveCubeNormalized`) (select `bool` _returnvalue :`false` (`KismetMathLibrary.MakeVector` 0.0 _returnvalue_2) :`true` (`KismetMathLibrary.MakeVector` _returnvalue_2)))
              (:`  `
                (bind (_direction _0_1) (`Timeline|MoveCubeNormalized` :!via `PlayFromStart` :!label _label_2)
                  (:`Update`
                    (if (< _0_1 0.0)
                      (`self.Stopped`)
                      (else
                        (`self.Trace Cube` (`KismetMathLibrary.VLerp` _return_start _return_end _0_1)))))
                  (:`Finished`
                    (`self.Stopped`))))))
          (:`then_1`
            (`GameplayStatics.SpawnSound2D` "/Game/Assets/Sounds/rock_slide_Cue.rock_slide_Cue" 1.0 1.0 0.0 null)))))))

(event `Stopped`
  (bind (_move_amount_x _move_amount_y _move_amount_z) (`KismetMathLibrary.BreakVector` (`self.Move Amount`)))
  (bind _attached_leaf (`self.Attached Leaf`))
  (`|ExecutionSequence`
    (:`then_0`
      (goto _label :!via `Reset`))
    (:`then_1`
      (goto _label_2 :!via `Stop`))
    (:`then_2`
      (bind _outhit (`KismetSystemLibrary.LineTraceSingle` (`self.K2_GetActorLocation`) (`KismetMathLibrary.TransformLocation` (`self.GetTransform`) (0.0 0.0 -400.0)) "TraceTypeQuery1"))
      (bind _returnvalue (`GameplayStatics.GetObjectClass` (`.HitActor` (`GameplayStatics.BreakHitResult` _outhit))))
      (if (or (== _returnvalue "/Game/Blueprints/BP_Water.BP_Water_C") (== _returnvalue "/Game/Blueprints/BP_WaterCurve.BP_WaterCurve_C"))
        (set `self.CanMove` false)
        (bind (_return_start _return_end) (`self.Set Playrate And Variables` (`self.MoveToWater`) (`KismetMathLibrary.MakeVector` 0.0 0.0 (- (* _move_amount_z -1.0) 5.0)))
          (:`  `
            (bind (_direction _0_1) (`Timeline|MoveToWater` :!via `PlayFromStart`)
              (:`Update`
                (`self.K2_SetActorLocation` (`KismetMathLibrary.VLerp` _return_start _return_end _0_1))))))))
    (:`then_3`
      (`/Engine/EditorBlueprintResources/StandardMacros.IsValid` _attached_leaf
        (:`Is Valid`
          (`/Game/Blueprints/BP_MovableLeaf.Stopped` _attached_leaf)
          (`self.K2_DetachFromActor` _attached_leaf "KeepWorld" "KeepWorld" "KeepWorld")
          (set `self.Attached Leaf` null))))))

(fn `UserConstructionScript`)
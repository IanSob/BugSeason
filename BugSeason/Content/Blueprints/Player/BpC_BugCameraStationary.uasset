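; Stationary bug camera Blueprint that responds to game-mode temperature changes by selecting among three post-process filters.
; A temperature change starts a blend to the matching filter, or sets the direction of one in progress forward or back via DeltaWeight.
; BeginPlay caches its offset in the bug character's local space.
; A helper uses that offset to test a distance against a threshold and compute a shifted box location.
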(event `self.ReceiveBeginPlay`
  ;[0.1264 1 0.2602] Set Some Default Variables
  (add `/Game/Blueprints/Player/BP_BugGamemode.Temperature Changed` (`/Game/Blueprints/UserFunctionLibrary.Get Bug Game Mode`) (delegate `Change LUT`))
  (set `self.Filter Array` (`|MakeArray` (`self.PP_1`) (`self.PP_2`) (`self.PP_3`)))
  (set `self.Current Filter` (`self.PP_1`))
  (bind _returnvalue (`GameplayStatics.GetActorOfClass` "/Game/Blueprints/Player/BP_BugCharacter.BP_BugCharacter_C"))
  (bind _output_get (set `self.BugCharacter` _returnvalue))
  (set `self.Square Local Offset` (`KismetMathLibrary.InverseTransformLocation` (`self.GetTransform` _output_get) (`self.K2_GetActorLocation`))))

(event `Change LUT`
  (params (NewTemp :type Integer))
  (bind _output (`|GetArrayItem` (`self.Filter Array`) NewTemp))
  ;[0.2125 0.5081 1] Update Filter Changes
  (if (`self.Lerping`)
    (if (== _output (`self.New Filter`))
      (set `self.DeltaWeight` 1 :!label _label)
      (elif (== _output (`self.Current Filter`))
        (set `self.DeltaWeight` -1)))
    (else
      (set `self.New Filter` _output)
      (set `self.Lerping` true)
      (goto _label))))

(fn `UserConstructionScript`)
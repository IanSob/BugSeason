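; Bug character camera that follows the player and switches post-process filters as the game's temperature changes.
; Game mode temperature events pick one of three filters, which Tick cross-fades by blend weight.
; A change back mid-blend reverses the fade, while a third filter requested then is ignored.
; Tick also checks the starting offset in character space per axis, moving the camera only when drift exceeds that axis's dead-zone threshold.
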(event `self.ReceiveBeginPlay`
  ;[0.1264 1 0.2602] Set Some Default Variables
  (add `/Game/Blueprints/Player/BP_BugGamemode.Temperature Changed` (`/Game/Blueprints/UserFunctionLibrary.Get Bug Game Mode`) (delegate `Change LUT`))
  (set `self.Filter Array` (`|MakeArray` (`self.PP_1`) (`self.PP_2`) (`self.PP_3`)))
  (set `self.Current Filter` (`self.PP_1`))
  (bind _returnvalue (`GameplayStatics.GetActorOfClass` "/Game/Blueprints/Player/BP_BugCharacter.BP_BugCharacter_C"))
  (bind _output_get (set `self.BugCharacter` _returnvalue))
  (set `self.Square Local Offset` (`KismetMathLibrary.InverseTransformLocation` (`self.GetTransform` _output_get) (`self.K2_GetActorLocation`))))

(event `Change LUT`
  (params (NewTemp :type Integer))
  (bind _output (`|GetArrayItem` (`self.Filter Array`) NewTemp))
  ;[0.2125 0.5081 1] Update Filter Changes
  (if (`self.Lerping`)
    (if (== _output (`self.New Filter`))
      (set `self.DeltaWeight` 1 :!label _label)
      (elif (== _output (`self.Current Filter`))
        (set `self.DeltaWeight` -1)))
    (else
      (set `self.New Filter` _output)
      (set `self.Lerping` true)
      (goto _label))))

(event `self.ReceiveTick`
  (params (DeltaSeconds :type "Float (single-precision)"))
  (bind (_returnvalue_x _returnvalue_y _returnvalue_z) (`KismetMathLibrary.BreakVector` (`self.K2_GetActorLocation`)))
  (bind (_returnvalue_x_2 _returnvalue_y_2) (`KismetMathLibrary.BreakVector` (`self.K2_GetActorLocation`)))
  (bind (_returnvalue_x_3 _returnvalue_y_3 _returnvalue_z_2) (`KismetMathLibrary.BreakVector` (`self.K2_GetActorLocation`)))
  (bind (_camera_movement_threshold_x _camera_movement_threshold_y _camera_movement_threshold_z) (`KismetMathLibrary.BreakVector` (`self.Camera Movement Threshold`)))
  (bind (_returnvalue_x_4 _returnvalue_y_4 _returnvalue_z_3) (`KismetMathLibrary.BreakVector` (- (`KismetMathLibrary.InverseTransformLocation` (`self.GetTransform` (`self.BugCharacter`)) (`self.K2_GetActorLocation`)) (`self.Square Local Offset`))))
  (`|ExecutionSequence`
    (:`then_0`
      ;[1 0.8112 0.3294] Update Blend Weights
      (if (`self.Lerping`)
        (bind _return_value (`/Game/Blueprints/BP_UserMacroLibrary.Lerp Over Time` 0.0 1.0 (`self.Transition Time`) (* DeltaSeconds (`self.DeltaWeight`)))
          (:`  `
            (set `PostProcessComponent.BlendWeight` (- 1.0 _return_value) (`self.Current Filter`))
            (set `PostProcessComponent.BlendWeight` _return_value (`self.New Filter`)))
          (:`Finished`
            (set `self.Lerping` false)
            (if (> (`self.DeltaWeight`) 0)
              (set `self.Current Filter` (`self.New Filter`)))))))
    (:`then_1`
      (`|ExecutionSequence`
        (:`then_0`
          (bind (_shouldmove _new_location) (`self.Find Box New Position` _returnvalue_x_4 _camera_movement_threshold_x)
            (:`  `
              (if _shouldmove
                (`self.K2_SetActorLocation` (`KismetMathLibrary.MakeVector` (.x _new_location) _returnvalue_y _returnvalue_z))))))
        (:`then_1`
          (bind (_shouldmove_2 _new_location_2) (`self.Find Box New Position` _returnvalue_y_4 _camera_movement_threshold_y)
            (:`  `
              (if _shouldmove_2
                (`self.K2_SetActorLocation` (`KismetMathLibrary.MakeVector` _returnvalue_x_3 (.y _new_location_2) _returnvalue_z_2))))))
        (:`then_2`
          (bind (_shouldmove_3 _new_location_3) (`self.Find Box New Position` _returnvalue_z_3 _camera_movement_threshold_z)
            (:`  `
              (if _shouldmove_3
                (`self.K2_SetActorLocation` (`KismetMathLibrary.MakeVector` _returnvalue_x_2 _returnvalue_y_2 (.z _new_location_3)))))))))))

(fn `UserConstructionScript`)
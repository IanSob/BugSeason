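; BugCamera is a player camera Blueprint that crossfades between three post-process filters as the game's temperature changes.
; On BeginPlay it binds to the bug game mode's temperature event, whose value indexes the filter array.
; Tick lerps the current and new filters' blend weights inversely over a transition time.
; Returning to the previous temperature mid-blend reverses the lerp through a signed delta weight, while a third filter is ignored.
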(event `self.ReceiveBeginPlay`
  ;[0.1264 1 0.2602] Set Some Default Variables
  (add `/Game/Blueprints/Player/BP_BugGamemode.Temperature Changed` (`/Game/Blueprints/UserFunctionLibrary.Get Bug Game Mode`) (delegate `Change LUT`))
  (set `self.Filter Array` (`|MakeArray` (`self.PP_1`) (`self.PP_2`) (`self.PP_3`)))
  (set `self.Current Filter` (`self.PP_1`)))

(event `Change LUT`
  (params (NewTemp :type Integer))
  (bind _output (`|GetArrayItem` (`self.Filter Array`) NewTemp))
  ;[0.2125 0.5081 1] Update Filter Changes
  (if (`self.Lerping`)
    (if (== _output (`self.New Filter`))
      (set `self.DeltaWeight` 1 :!label _label)
      (elif (== _output (`self.Current Filter`))
        (set `self.DeltaWeight` -1)))
    (else
      (set `self.New Filter` _output)
      (set `self.Lerping` true)
      (goto _label))))

(event `self.ReceiveTick`
  (params (DeltaSeconds :type "Float (single-precision)"))
  ;[1 0.8112 0.3294] Update Blend Weights
  (if (`self.Lerping`)
    (bind _return_value (`/Game/Blueprints/UserMacroLibrary.Lerp Over Time` 0.0 1.0 (`self.Transition Time`) (* DeltaSeconds (`self.DeltaWeight`)))
      (:`  `
        (set `PostProcessComponent.BlendWeight` (- 1.0 _return_value) (`self.Current Filter`))
        (set `PostProcessComponent.BlendWeight` _return_value (`self.New Filter`)))
      (:`Finished`
        (set `self.Lerping` false)
        (if (> (`self.DeltaWeight`) 0)
          (set `self.Current Filter` (`self.New Filter`)))))))

(fn `UserConstructionScript`)
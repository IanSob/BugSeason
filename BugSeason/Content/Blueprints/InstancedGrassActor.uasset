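; Instanced grass actor whose wind sway reacts to temperature changes broadcast by the bug game mode.
; On BeginPlay it subscribes to that change and gives each instanced static mesh component a dynamic material instance for slot 0, caching them in an array.
; Each temperature change pushes wave and speed scalar parameters to all cached materials, using a stronger windy preset for one temperature state and calmer defaults otherwise.
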(event `self.ReceiveBeginPlay`
  (add `/Game/Blueprints/Player/BP_BugGamemode.Temperature Changed` (`/Game/Blueprints/UserFunctionLibrary.Get Bug Game Mode`) (delegate `Temperature Change`))
  (for _array_element (`self.K2_GetComponentsByClass` "/Script/Engine.InstancedStaticMeshComponent")
    (bind _returnvalue (`PrimitiveComponent.CreateDynamicMaterialInstance` _array_element 0 (`PrimitiveComponent.GetMaterial` _array_element 0) "None"))
    (`KismetArrayLibrary.Array_Add` (`self.Material Instances Array`) _returnvalue)
    (`PrimitiveComponent.SetMaterial` _array_element 0 _returnvalue)))

(event `Temperature Change`
  (params (NewTemp :type Integer))
  (switch `int` NewTemp
    (:`Default`
      ;[1 1 1] Default Wind Speeds
      (`self.Change Wind Speed` 10.0 5.0 3.0 1.0))
    (:`1`
      ;[1 1 1] Windy
      (`self.Change Wind Speed` 20.0 10.0 10.0 5.0))))

(fn `UserConstructionScript`)
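; Blueprint function library with shared helpers for the bug game.
; GetBugGameMode returns the current game mode cast to BP_BugGamemode.
; SwapObjects exchanges two by-reference object variables through a temporary, only when both objects share the same class.
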(fn `Get Bug Game Mode`
  (returns (`Return Value` :type "/Game/Player/BP_BugGamemode Object Reference"))
  (bind _asbp_bug_gamemode (cast `/Game/Player/BP_BugGamemode` (`GameplayStatics.GetGameMode` null))
    (:`then`
      (return _asbp_bug_gamemode))
    (:`CastFailed`
      (return null))))

(fn `Swap Objects`
  (params (`Object 1` :type "Object Object Reference (by ref)") (`Object 2` :type "Object Object Reference (by ref)"))
  (locals (`Temp Object` :type "Object Object Reference"))
  (if (== (`GameplayStatics.GetObjectClass` `Object 1`) (`GameplayStatics.GetObjectClass` `Object 2`))
    (bind _output_get (set `local.Temp Object` `Object 1`))
    (`|VariableSetRef` `Object 1` `Object 2`)
    (`|VariableSetRef` `Object 2` _output_get)
    (return)
    (else
      (return))))
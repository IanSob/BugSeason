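; BP_TempatureShroom is a mushroom that changes the bug game's temperature when the BP_BugCharacter hits it.
; If CanChangeTemp is set, a hit plays a squish sound and sends its Temperature to the game mode, or zero if that value is already active.
; The MushroomGlow timeline plays or reverses to drive a Glowy parameter on a dynamic material.
; A DoOnce with delayed reset limits repeat triggers.
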(event `self.ReceiveBeginPlay`
  (bind _returnvalue (`KismetMaterialLibrary.CreateDynamicMaterialInstance` "/Game/Assets/Materials/M_Shrooms.M_Shrooms"))
  (bind _output_get (set `self.Shroom Material` _returnvalue))
  (`PrimitiveComponent.SetMaterial` (`self.Plane`) 0 _output_get))

(event `self.ReceiveHit`
  (params (MyComp :type "PrimitiveComponent Object Reference") (Other :type "Actor Object Reference") (OtherComp :type "PrimitiveComponent Object Reference") (bSelfMoved :type Boolean) (HitLocation :type "Vector Structure") (HitNormal :type "Vector Structure") (NormalImpulse :type "Vector Structure") (Hit :type "HitResult Structure (by ref)"))
  (bind _return_value (`/Game/Blueprints/UserFunctionLibrary.Get Bug Game Mode`))
  (bind _mushroomglow (`self.MushroomGlow`))
  (cast `/Game/Blueprints/Player/BP_BugCharacter` Other)
  (if (`self.CanChangeTemp`)
    (`/Engine/EditorBlueprintResources/StandardMacros.DoOnce` false :!label _label
      (:`Completed`
        (`GameplayStatics.PlaySound2D` "/Game/Assets/Sounds/shroom_squish_Cue.shroom_squish_Cue" 1.0 1.0 0.0 null null)
        (bind _temperature (`/Game/Blueprints/Player/BP_BugGamemode.Get Temperature` (`/Game/Blueprints/UserFunctionLibrary.Get Bug Game Mode`)))
        (if (== _temperature (`self.Temperature`))
          (`/Game/Blueprints/Player/BP_BugGamemode.Change Temperature` _return_value 0)
          (`TimelineComponent.Reverse` _mushroomglow)
          (else
            (`/Game/Blueprints/Player/BP_BugGamemode.Change Temperature` _return_value (`self.Temperature`))
            (`TimelineComponent.Play` _mushroomglow)))
        (`KismetSystemLibrary.Delay` 5.0)
        (goto _label :!via `Reset`)))))

(fn `UserConstructionScript`)
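; Pushable rock that slides one tile along local X or Y, away from a grounded BP_BugCharacter touching its XMove or YMove trigger.
; BeginPlay fills any zero MoveAmount axis with twice the box extent.
; MoveRock (Y) and MoveRock_2 (X) compare local positions to choose direction, line trace for obstacles, then ease the Box with MoveComponentTo, guarded by Moving.
; The negative X trace checks along negative Y instead.
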(event `self.ReceiveBeginPlay`
  (bind (_move_amount_x _move_amount_y _move_amount_z) (`KismetMathLibrary.BreakVector` (`self.Move Amount`)))
  (bind (_move_amount_x_2 _move_amount_y_2 _move_amount_z_2) (`KismetMathLibrary.BreakVector` (`self.Move Amount`)))
  (bind (_returnvalue_x _returnvalue_y _returnvalue_z) (`KismetMathLibrary.BreakVector` (* (`BoxComponent.GetUnscaledBoxExtent` (`self.Box`)) (2.0 2.0 2.0))))
  ;[1 1 1] Yes, I Know This Is Really Ugly Code
  (`|ExecutionSequence`
    (:`then_0`
      (if (== _move_amount_x 0.0)
        (set `self.Move Amount` (`KismetMathLibrary.MakeVector` _returnvalue_x _move_amount_y_2 _move_amount_z_2))))
    (:`then_1`
      (if (== _move_amount_y 0.0)
        (set `self.Move Amount` (`KismetMathLibrary.MakeVector` _move_amount_x_2 _returnvalue_y _move_amount_z_2))))
    (:`then_2`
      (if (== _move_amount_z 0.0)
        (set `self.Move Amount` (`KismetMathLibrary.MakeVector` _move_amount_x_2 _move_amount_y_2 _returnvalue_z))))))

(event `self.Y Move.OnComponentBeginOverlap`
  (params (OverlappedComponent :type "PrimitiveComponent Object Reference") (OtherActor :type "Actor Object Reference") (OtherComp :type "PrimitiveComponent Object Reference") (OtherBodyIndex :type Integer) (bFromSweep :type Boolean) (SweepResult :type "HitResult Structure (by ref)"))
  (bind (_move_amount_x _move_amount_y) (`KismetMathLibrary.BreakVector` (`self.Move Amount`)))
  (bind _box (`self.Box`))
  (bind _box_2 (`self.Box`))
  (bind (_move_amount_x_2 _move_amount_y_2) (`KismetMathLibrary.BreakVector` (`self.Move Amount`)))
  (bind _box_3 (`self.Box`))
  (bind _box_4 (`self.Box`))
  (bind (_move_amount_x_3 _move_amount_y_3) (`KismetMathLibrary.BreakVector` (`self.Move Amount`)))
  (bind (_move_amount_x_4 _move_amount_y_4) (`KismetMathLibrary.BreakVector` (`self.Move Amount`)))
  (bind (_relativelocation_x _relativelocation_y) (`KismetMathLibrary.BreakVector` (`SceneComponent.RelativeLocation` (`self.Box`))))
  (bind (_returnvalue_x _returnvalue_y) (`KismetMathLibrary.BreakVector` (`KismetMathLibrary.InverseTransformLocation` (`SceneComponent.K2_GetComponentToWorld` (`self.DefaultSceneRoot`)) (`self.K2_GetActorLocation` OtherActor))))
  (bind _asbp_bug_character (cast `/Game/Blueprints/Player/BP_BugCharacter` OtherActor))
  (if (`NavMovementComponent.IsMovingOnGround` (`Character.CharacterMovement` _asbp_bug_character))
    (if (and (== (`GameplayStatics.GetObjectClass` OtherComp) "/Script/Engine.CapsuleComponent") (== (`GameplayStatics.GetObjectClass` OtherActor) "/Game/Blueprints/Player/BP_BugCharacter.BP_BugCharacter_C"))
      (if (not (`self.Moving`))
        (set `self.Moving` true)
        (if (< _returnvalue_y _relativelocation_y)
          (bind (_outhit _returnvalue) (`KismetSystemLibrary.LineTraceSingle` (`SceneComponent.K2_GetComponentLocation` _box) (`KismetMathLibrary.TransformLocation` (`SceneComponent.K2_GetComponentToWorld` (`self.DefaultSceneRoot`)) (+ (`SceneComponent.RelativeLocation` _box) (`KismetMathLibrary.MakeVector` 0.0 _move_amount_y))) "TraceTypeQuery1"))
          (if (not _returnvalue)
            (`KismetSystemLibrary.MoveComponentTo` _box_3 (+ (`SceneComponent.RelativeLocation` _box_3) (`KismetMathLibrary.MakeVector` 0.0 _move_amount_y_4)) (`SceneComponent.RelativeRotation` _box_3) true true (`self.Time To Move One Tile`)))
          (set `self.Moving` false)
          (else
            (bind (_outhit_2 _returnvalue_2) (`KismetSystemLibrary.LineTraceSingle` (`SceneComponent.K2_GetComponentLocation` _box_2) (`KismetMathLibrary.TransformLocation` (`SceneComponent.K2_GetComponentToWorld` (`self.DefaultSceneRoot`)) (- (`SceneComponent.RelativeLocation` _box_2) (`KismetMathLibrary.MakeVector` 0.0 _move_amount_y_2))) "TraceTypeQuery1"))
            (if (not _returnvalue_2)
              (`KismetSystemLibrary.MoveComponentTo` _box_4 (- (`SceneComponent.RelativeLocation` _box_4) (`KismetMathLibrary.MakeVector` 0.0 _move_amount_y_3)) (`SceneComponent.RelativeRotation` _box_4) true true (`self.Time To Move One Tile`)))
            (set `self.Moving` false)))))))

(event `self.X Move.OnComponentBeginOverlap`
  (params (OverlappedComponent :type "PrimitiveComponent Object Reference") (OtherActor :type "Actor Object Reference") (OtherComp :type "PrimitiveComponent Object Reference") (OtherBodyIndex :type Integer) (bFromSweep :type Boolean) (SweepResult :type "HitResult Structure (by ref)"))
  (bind _move_amount_x (`KismetMathLibrary.BreakVector` (`self.Move Amount`)))
  (bind _box (`self.Box`))
  (bind _box_2 (`self.Box`))
  (bind (_move_amount_x_2 _move_amount_y) (`KismetMathLibrary.BreakVector` (`self.Move Amount`)))
  (bind _box_3 (`self.Box`))
  (bind _box_4 (`self.Box`))
  (bind _move_amount_x_3 (`KismetMathLibrary.BreakVector` (`self.Move Amount`)))
  (bind _move_amount_x_4 (`KismetMathLibrary.BreakVector` (`self.Move Amount`)))
  (bind _relativelocation_x (`KismetMathLibrary.BreakVector` (`SceneComponent.RelativeLocation` (`self.Box`))))
  (bind _returnvalue_x (`KismetMathLibrary.BreakVector` (`KismetMathLibrary.InverseTransformLocation` (`SceneComponent.K2_GetComponentToWorld` (`self.DefaultSceneRoot`)) (`self.K2_GetActorLocation` OtherActor))))
  (bind _asbp_bug_character (cast `/Game/Blueprints/Player/BP_BugCharacter` OtherActor))
  (if (`NavMovementComponent.IsMovingOnGround` (`Character.CharacterMovement` _asbp_bug_character))
    (if (and (== (`GameplayStatics.GetObjectClass` OtherComp) "/Script/Engine.CapsuleComponent") (== (`GameplayStatics.GetObjectClass` OtherActor) "/Game/Blueprints/Player/BP_BugCharacter.BP_BugCharacter_C"))
      (if (not (`self.Moving`))
        (set `self.Moving` true)
        (if (< _returnvalue_x _relativelocation_x)
          (bind (_outhit _returnvalue) (`KismetSystemLibrary.LineTraceSingle` (`SceneComponent.K2_GetComponentLocation` _box) (`KismetMathLibrary.TransformLocation` (`SceneComponent.K2_GetComponentToWorld` (`self.DefaultSceneRoot`)) (+ (`SceneComponent.RelativeLocation` _box) (`KismetMathLibrary.MakeVector` _move_amount_x))) "TraceTypeQuery1"))
          (if (not _returnvalue)
            (`KismetSystemLibrary.MoveComponentTo` _box_3 (+ (`SceneComponent.RelativeLocation` _box_3) (`KismetMathLibrary.MakeVector` _move_amount_x_4)) (`SceneComponent.RelativeRotation` _box_3) true true (`self.Time To Move One Tile`)))
          (set `self.Moving` false)
          (else
            (bind (_outhit_2 _returnvalue_2) (`KismetSystemLibrary.LineTraceSingle` (`SceneComponent.K2_GetComponentLocation` _box_2) (`KismetMathLibrary.TransformLocation` (`SceneComponent.K2_GetComponentToWorld` (`self.DefaultSceneRoot`)) (- (`SceneComponent.RelativeLocation` _box_2) (`KismetMathLibrary.MakeVector` 0.0 _move_amount_y))) "TraceTypeQuery1"))
            (if (not _returnvalue_2)
              (`KismetSystemLibrary.MoveComponentTo` _box_4 (- (`SceneComponent.RelativeLocation` _box_4) (`KismetMathLibrary.MakeVector` _move_amount_x_3)) (`SceneComponent.RelativeRotation` _box_4) true true (`self.Time To Move One Tile`)))
            (set `self.Moving` false)))))))

(fn `UserConstructionScript`)
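; BP_MovableLeaf is a leaf actor that moves by set offsets, defaulting to its box size, and drops onto water.
; When stopped, it traces downward for water actors, disables movement and lerps down on a timeline whose play rate scales with distance for constant speed.
; A Trace Cube helper box-traces moves and reverses the movement timeline on blocking hits.
; Overlapping any non-ignored class destroys the leaf.
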(event `self.ReceiveBeginPlay`
  (bind (_move_amount_x _move_amount_y _move_amount_z) (`KismetMathLibrary.BreakVector` (`self.Move Amount`)))
  (bind (_move_amount_x_2 _move_amount_y_2 _move_amount_z_2) (`KismetMathLibrary.BreakVector` (`self.Move Amount`)))
  (bind (_returnvalue_x _returnvalue_y _returnvalue_z) (`KismetMathLibrary.BreakVector` (* (`BoxComponent.GetUnscaledBoxExtent` (`self.Box`)) (2.0 2.0 2.0))))
  ;[1 1 1] Yes, I Know This Is Really Ugly Code
  (`|ExecutionSequence`
    (:`then_0`
      (if (== _move_amount_x 0.0)
        (set `self.Move Amount` (`KismetMathLibrary.MakeVector` _returnvalue_x _move_amount_y_2 _move_amount_z_2))))
    (:`then_1`
      (if (== _move_amount_y 0.0)
        (set `self.Move Amount` (`KismetMathLibrary.MakeVector` _move_amount_x_2 _returnvalue_y _move_amount_z_2))))
    (:`then_2`
      (if (== _move_amount_z 0.0)
        (set `self.Move Amount` (`KismetMathLibrary.MakeVector` _move_amount_x_2 _move_amount_y_2 _returnvalue_z))))
    (:`then_3`
      (`KismetSystemLibrary.PrintString` "Hello"))))

(event `Stopped`
  (bind (_move_amount_x _move_amount_y _move_amount_z) (`KismetMathLibrary.BreakVector` (`self.Move Amount`)))
  (bind _outhit (`KismetSystemLibrary.LineTraceSingle` (`self.K2_GetActorLocation`) (`KismetMathLibrary.TransformLocation` (`self.GetTransform`) (0.0 0.0 -400.0)) "TraceTypeQuery1"))
  (bind _returnvalue (`GameplayStatics.GetObjectClass` (`.HitActor` (`GameplayStatics.BreakHitResult` _outhit))))
  (if (or (== _returnvalue "/Game/Blueprints/BP_Water.BP_Water_C") (== _returnvalue "/Game/Blueprints/BP_WaterCurve.BP_WaterCurve_C"))
    (set `self.CanMove` false)
    (bind (_return_start _return_end) (`self.Set Playrate And Variables` (`self.MoveToWater`) (`KismetMathLibrary.MakeVector` 0.0 0.0 (- (* _move_amount_z -1.0) 5.0)))
      (:`  `
        (bind (_direction _0_1) (`Timeline|MoveToWater` :!via `PlayFromStart`)
          (:`Update`
            (`self.K2_SetActorLocation` (`KismetMathLibrary.VLerp` _return_start _return_end _0_1))))))))

(event `self.ReceiveActorBeginOverlap`
  (params (OtherActor :type "Actor Object Reference"))
  (bind _returnvalue (`GameplayStatics.GetObjectClass` OtherActor))
  ;[1 1 1] Check for ignored classes
  (if (not (`/Game/Blueprints/UserFunctionLibrary.==InClassArray` (`self.Ignored Classes`) _returnvalue))
    (`self.K2_DestroyActor`)
    (`KismetSystemLibrary.PrintString` (`KismetSystemLibrary.GetClassDisplayName` _returnvalue))))

(fn `UserConstructionScript`)
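; BPTempatureShroom is an interactable mushroom that toggles the game's temperature.
; On releasing the Interact input while CanChangeTemp is true, it plays a squish sound and reads the current temperature from the bug game mode.
; If that already equals the shroom's own Temperature value it resets the temperature to zero; otherwise it sets it to that value.
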(event `InputAction|Interact`
  (params (Key :type "Key Structure"))
  (bind _return_value (`/Game/Blueprints/UserFunctionLibrary.Get Bug Game Mode`))
  (:`Released`
    (if (`self.CanChangeTemp`)
      (`GameplayStatics.PlaySound2D` "/Game/Assets/Sounds/shroom_squish_Cue.shroom_squish_Cue" 1.0 1.0 0.0 null null)
      (bind _temperature (`/Game/Blueprints/Player/BP_BugGamemode.Get Temperature` (`/Game/Blueprints/UserFunctionLibrary.Get Bug Game Mode`)))
      (if (== _temperature (`self.Temperature`))
        (`/Game/Blueprints/Player/BP_BugGamemode.Change Temperature` _return_value 0)
        (else
          (`/Game/Blueprints/Player/BP_BugGamemode.Change Temperature` _return_value (`self.Temperature`)))))))

(fn `UserConstructionScript`)
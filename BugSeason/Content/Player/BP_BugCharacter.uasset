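; BP_BugCharacter is a player character Blueprint for a bug that walks and jumps on Space.
; Each tick it turns the GetWS and GetAD axis values into an actor-relative direction and feeds it to CharacterMovement as input.
; UpdateCamera sets control rotation to a given camera yaw while keeping the actor's pitch and roll.
; BeginPlay calls it with the first BugCamera's rotation, if one exists.
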(event `self.ReceiveBeginPlay`
  (bind _outactors (`GameplayStatics.GetAllActorsOfClass` "/Game/Player/BugCamera.BugCamera_C"))
  (if (> (`KismetArrayLibrary.Array_Length` _outactors) 0)
    (`self.Update Camera` (`self.K2_GetActorRotation` (`|GetArrayItem` _outactors)))))

(event `Key|SpaceBar`
  (params (Key :type "Key Structure"))
  (:`Pressed`
    (`self.Jump`)))

(event `self.ReceiveTick`
  (params (DeltaSeconds :type "Float (single-precision)"))
  (bind _returnvalue (`self.GetTransform` self))
  (`PawnMovementComponent.AddInputVector` (`self.CharacterMovement`) (- (`KismetMathLibrary.TransformLocation` _returnvalue (`KismetMathLibrary.MakeVector` (`self.GetInputAxisValue`) (`self.GetInputAxisValue`))) (`KismetMathLibrary.TransformLocation` _returnvalue)) false))

(event `Update Camera`
  (params (`Camera Rotation` :type "Rotator Structure"))
  (bind (_returnvalue_roll _returnvalue_pitch) (`KismetMathLibrary.BreakRotator` (`self.K2_GetActorRotation`)))
  (`Controller.SetControlRotation` (`self.GetController`) (`KismetMathLibrary.MakeRotator` _returnvalue_roll _returnvalue_pitch `Camera Rotation_Yaw`)))

(fn `UserConstructionScript`)